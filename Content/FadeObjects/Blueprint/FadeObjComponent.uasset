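; Component that fades objects blocking the camera's view of characters of a given class.
; A looping timer capsule-traces from camera to each character, keeping hits that pass a distance or near-camera check.
; FadeMakeArray swaps their materials for FadeMaterial dynamic instances, ignores Camera collision and flags objects no longer hit.
; A faster timer interpolates the Fade parameter, restoring materials and collision once fully opaque.
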(event Custom|FadeObjCalculate_Start
  ;[0.9705 1 0] Objects Fade effect between actor and camera
  ;;[0 1 0.5877] FadeObjWorker
  (bind _returnvalue (Utilities|Time|SetTimerbyEvent (delegate Custom|FadeObjWorker) 0.05 true))
  (Variables|Default|SetFadeObjCalculateTimer _returnvalue))

(event Custom|AddObjectsToHide
  (bind _returnvalue (Game|GetPlayerCameraManager 0))
  (bind _returnvalue_2 (Camera|GetCameraLocation _returnvalue))
  ;[0.9705 1 0] Objects Fade effect between actor and camera
  (Utilities|Time|SetTimerbyEvent (delegate Custom|AddObjectsToHide) 0.1 true)
  ;;[0 1 0.1257] Fade objects between camera and this class
  (bind _outactors (Actor|GetAllActorsOfClass (Variables|SetThisOptions|GetCharactersClass)))
  (for _array_element _outactors
    (bind (_outhits _returnvalue_3) (Class|KismetSystemLibrary|CapsuleTraceMultiforObjects _returnvalue_2 (Transformation|GetActorLocation _array_element) (Variables|SetThisOptions|GetCapsuleRadius) (Variables|SetThisOptions|GetCapsuleHalfHeight) (Variables|SetThisOptions|GetObjectsType) false (Variables|SetThisOptions|GetActorsToIgnore) "None" true))
    (if _returnvalue_3
      (for _array_element_2 _outhits
        (bind _outactors_2 (Collision|SphereOverlapActors _returnvalue_2 (Variables|SetThisOptions|GetNearCameraRadius) (Variables|SetThisOptions|GetObjectsType) 0 (Variables|SetThisOptions|GetActorsToIgnore)))
        (if (or (< (Math|Vector|VectorLength (- _returnvalue_2 (Transformation|GetActorLocation _array_element))) (Variables|SetThisOptions|GetDistance)) (Utilities|Array|ContainsItem _outactors_2 (.HitActor (Collision|BreakHitResult _array_element_2))))
          (Utilities|Array|AddUnique (Variables|Default|GetFadeObjectsHit) (.HitComponent (Collision|BreakHitResult _array_element_2)))))))
  ;;[1 0 0.8988] Make fade objects array
  (CallFunction|FadeMakeArray))

(event Custom|FadeObjWorker
  (bind _fadeobjects (Variables|Default|GetFadeObjects))
  (bind _fadeobjects_2 (Variables|Default|GetFadeObjects))
  ;[0.9705 1 0] Objects Fade effect between actor and camera
  ;;[0 1 0.5877] FadeObjWorker
  (if (> (Utilities|Array|Length (Variables|Default|GetFadeObjects)) 0)
    (for (_array_element _array_index) _fadeobjects_2
      (Variables|Default|SetFadeNowID _array_index)
      (for _array_element_2 (.MID_Fade (Utilities|Struct|BreakFadeObjStruct _array_element))
        (Rendering|Material|SetScalarParameterValue _array_element_2 "Fade" (Math|Interpolation|FInterptoConstant (.FadeCurrent (Utilities|Struct|BreakFadeObjStruct _array_element)) (select (.toHide (Utilities|Struct|BreakFadeObjStruct _array_element)) (select (== _array_index (Utilities|Array|LastIndex _fadeobjects_2)) 0.3 0.1) 1.0) (Utilities|Time|GetWorldDeltaSeconds) (Variables|SetThisOptions|GetFadeRate)) :!class /Script/Engine.MaterialInstanceDynamic)
        (bind _output_get (Variables|Default|SetCurrentFade (Math|Interpolation|FInterptoConstant (.FadeCurrent (Utilities|Struct|BreakFadeObjStruct _array_element)) (select (.toHide (Utilities|Struct|BreakFadeObjStruct _array_element)) (select (== _array_index (Utilities|Array|LastIndex _fadeobjects_2)) 0.3 0.1) 1.0) (Utilities|Time|GetWorldDeltaSeconds) (Variables|SetThisOptions|GetFadeRate))))
        (Utilities|Array|SetArrayElem _fadeobjects (Variables|Default|GetFadeNowID) (Utilities|FadeConnectMacroFB (Utilities|Array|Get(acopy) _fadeobjects (Variables|Default|GetFadeNowID)) _output_get (.toHide (Utilities|Struct|BreakFadeObjStruct _array_element)))))
      ;;;[1 1 1] Remove index
      (if (== (Variables|Default|GetCurrentFade) 1.0)
        (for (_array_element_3 _array_index_2) (.basematerialinterface (Utilities|Array|Get(acopy) (Variables|Default|GetFadeObjects) (Variables|Default|GetFadeNowID)))
          (Rendering|Material|SetMaterial (.primitivecomponent (Utilities|Array|Get(acopy) (Variables|Default|GetFadeObjects) (Variables|Default|GetFadeNowID))) _array_index_2 _array_element_3))
        (Collision|SetCollisionResponsetoChannel (.primitivecomponent (Utilities|Array|Get(acopy) (Variables|Default|GetFadeObjects) (Variables|Default|GetFadeNowID))) "ECC_Camera" "ECR_Block")
        (Utilities|Array|RemoveIndex (Variables|Default|GetFadeObjects) (Variables|Default|GetFadeNowID))
        (Utilities|Array|RemoveIndex (Variables|Default|GetFadeObjectsTemp) (Variables|Default|GetFadeNowID))))))

(event EventBeginPlay
  ;[0 0.4096 1] Init
  (if (Variables|SetThisOptions|GetbIsEnabale)
    (CallFunction|FadeObjCalculateStart)
    (CallFunction|AddObjectstoHide)))

(fn FadeMakeArray
  (bind _fadeobjects (Variables|Default|GetFadeObjects))
  (for _array_element (Variables|Default|GetFadeObjectsHit)
    (if (not (Utilities|Array|ContainsItem (Variables|Default|GetFadeObjectsTemp) _array_element))
      (Utilities|Array|Clear (LocalVariables|GetL_MID_Materials))
      (Utilities|Array|Clear (LocalVariables|GetL_BaseMaterials))
      (Utilities|Array|AddUnique (Variables|Default|GetFadeObjectsTemp) _array_element)
      (for _index (range 0 (Rendering|Material|GetNumMaterials _array_element))
        (bind _returnvalue (Rendering|Material|CreateDynamicMaterialInstance (Variables|Default|GetFadeMaterial) "None" :!class /Script/Engine.KismetMaterialLibrary))
        (Utilities|Array|Add (LocalVariables|GetL_MID_Materials) _returnvalue)
        (Utilities|Array|Add (LocalVariables|GetL_BaseMaterials) (Rendering|Material|GetMaterial _array_element _index))
        (Rendering|Material|SetMaterial _array_element _index _returnvalue))
      (Utilities|Array|Add (Variables|Default|GetFadeObjects) (Utilities|Struct|MakeFadeObjStruct _array_element (LocalVariables|GetL_BaseMaterials) (LocalVariables|GetL_MID_Materials) 1.0 true))
      (Collision|SetCollisionResponsetoChannel _array_element "ECC_Camera" "ECR_Ignore")))
  (for (_array_element_2 _array_index) (Variables|Default|GetFadeObjectsTemp)
    (if (not (Utilities|Array|ContainsItem (Variables|Default|GetFadeObjectsHit) _array_element_2))
      (Utilities|Array|SetArrayElem _fadeobjects _array_index (Utilities|FadeConnectMacroB (Utilities|Array|Get(acopy) _fadeobjects _array_index) false))))
  (Utilities|Array|Clear (Variables|Default|GetFadeObjectsHit))
  (return))