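; Third-person dog player character that barks, sprints and carries objects in its mouth, with helpers to rotate and reset the camera.
; Grab sphere-traces for Cylinders physics actors, awards points and holds them via a physics handle that follows GrabLocation each tick until Drop.
; Tick also compares horizontal distance to HumanCameraLocation, adding GameMode energy inside RadiusBorder and draining it beyond CatchBorder.
; Bark emits AI noise and plays audio; BlowHorn is an empty stub.
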(event Custom|CompareCameraAndDogLocation
  ;[0.4002 1 0.3448] Energy By Radius
  ;;[1 1 1] Compare Camera and charecter location
  (bind _output_get (Variables|Default|SetCameraAndDogDistance (- (Variables|Default|GetHumanCameraLocation) (Transformation|GetWorldLocation (Variables|Character|GetMesh)))))
  (bind _output_get_2 (Variables|Default|SetAllTogetherDistance (Math|Float|Sqrt (+ (Math|Float|Square (Math|Float|Absolute(Float) (.x _output_get))) (Math|Float|Square (Math|Float|Absolute(Float) (.y _output_get)))))))
  ;;;[1 1 1] Compare Camera and charecter location
  (if (> _output_get_2 (Variables|Default|GetRadiusBorder))
    (if (> (Variables|Default|GetAllTogetherDistance) (Variables|Default|GetCatchBorder))
      (Variables|Default|SetIsInsideRadius false)
      ;;;[1 1 1] Reduce energy
      (if (>= (- (Variables|/Game/Shenanidog/BluePrints/GameFiles/BP_Game_Mode_Base.BP_Game_Mode_Base_C|GetEnergyAmount (Variables|Default|GetBP_GameMode%20ref)) (Variables|Default|GetEnergy%20to%20Reduce)) 0.0)
        (Variables|/Game/Shenanidog/BluePrints/GameFiles/BP_Game_Mode_Base.BP_Game_Mode_Base_C|SetEnergyAmount (Variables|Default|GetBP_GameMode%20ref) (- (Variables|/Game/Shenanidog/BluePrints/GameFiles/BP_Game_Mode_Base.BP_Game_Mode_Base_C|GetEnergyAmount (Variables|Default|GetBP_GameMode%20ref)) (Variables|Default|GetEnergy%20to%20Reduce)))
        (Default|UpdateUI (Variables|Default|GetBP_GameMode%20ref))))
    (else
      (Variables|Default|SetIsInsideRadius true)
      ;;[1 1 1] Add energy
      (if (<= (+ (Variables|/Game/Shenanidog/BluePrints/GameFiles/BP_Game_Mode_Base.BP_Game_Mode_Base_C|GetEnergyAmount (Variables|Default|GetBP_GameMode%20ref)) (Variables|Default|GetEnergy%20to%20Add)) (+ (Variables|/Game/Shenanidog/BluePrints/GameFiles/BP_Game_Mode_Base.BP_Game_Mode_Base_C|GetMaxEnergyAmount (Variables|Default|GetBP_GameMode%20ref)) 2e+01))
        (Variables|/Game/Shenanidog/BluePrints/GameFiles/BP_Game_Mode_Base.BP_Game_Mode_Base_C|SetEnergyAmount (Variables|Default|GetBP_GameMode%20ref) (+ (Variables|/Game/Shenanidog/BluePrints/GameFiles/BP_Game_Mode_Base.BP_Game_Mode_Base_C|GetEnergyAmount (Variables|Default|GetBP_GameMode%20ref)) (Variables|Default|GetEnergy%20to%20Add)))
        (Default|UpdateUI (Variables|Default|GetBP_GameMode%20ref))))))

(event EventBeginPlay
  ;[1 1 1] Cast to BP_GameMode
  (bind _asbp_game_mode_base (Utilities|Casting|CastToBP_Game_Mode_Base (Game|GetGameMode)))
  (Variables|Default|SetBP_GameMode%20ref _asbp_game_mode_base))

(event Collision|EventActorBeginOverlap
  (params (OtherActor :type Actor%20Object%20Reference)))

(event EventTick
  (params (DeltaSeconds :type Float%20%28single-precision%29))
  ;[1 1 1] UpdateGrabLocation every frame - mouth grab - grab location
  (Physics|Components|PhysicsHandle|SetTargetLocation (Variables|Default|GetMouthGrab) (Transformation|GetWorldLocation (Variables|Default|GetGrabLocation)))
  (CallFunction|CompareCameraandDogLocation))

(event Input|ActionEvents|InputActionBark
  (params (Key :type Key%20Structure :default "None"))
  ;[1 1 1] Bark activation & release
)

(fn ConstructionScript)

(fn UpdateMovementSpeed
  (bind _charactermovement (Variables|Character|GetCharacterMovement))
  (if (Variables|Default|GetIsSprinting)
    (Variables|/Script/Engine.CharacterMovementComponent|SetMaxWalkSpeed _charactermovement 7.5e+02)
    (else
      (Variables|/Script/Engine.CharacterMovementComponent|SetMaxWalkSpeed _charactermovement 5e+02))))

(fn BlowHorn
  ;[1 1 1] Blow Force Event
)

(fn Grab
  (bind _mouthforgrab (Variables|Default|GetMouthForGrab))
  (bind _mesh (Variables|Character|GetMesh))
  (bind _returnvalue (Transformation|GetWorldLocation _mouthforgrab))
  ;[1 1 1] We recognize from sphere of trace for object , what did we hit , and move the hit object to the grab component
  (bind (_outhit _returnvalue_2) (Collision|SphereTraceForObjects _returnvalue (+ _returnvalue (* (Math|Vector|GetForwardVector _mouthforgrab) 5e+01)) 5e+01 (Utilities|Array|MakeArray "ObjectTypeQuery4") false 0 "None"))
  (if _returnvalue_2
    (bind _ascylinders (Utilities|Casting|CastToCylinders (.HitActor (Collision|BreakHitResult _outhit)))
      (:then
        (Variables|Default|SetCylindersRef 0)
        (Class|PhysicsHandleComponent|GrabComponentatLocation (Variables|Default|GetMouthGrab) (.HitComponent (Collision|BreakHitResult _outhit)) (Class|SkinnedMeshComponent|GetBoneName _mesh (Class|SkinnedMeshComponent|GetBoneIndex _mesh "mouth")) (Transformation|GetWorldLocation (.HitComponent (Collision|BreakHitResult _outhit))))
        ;;[1 1 1] This is if we dont want the object we grab colliding with use
        (Collision|SetCollisionResponsetoChannel (.HitComponent (Collision|BreakHitResult _outhit)) "ECC_Pawn" "ECR_Ignore")
        (Variables|Default|SetIsGrabing true)
        (Default|UpdatetheUIforScore _ascylinders (Variables|/Game/Shenanidog/BluePrints/Objects/Cylinders.Cylinders_C|GetPointsForGrab _ascylinders))
        (Class|TogglesInterface|ToggleGrab(Message) (.HitActor (Collision|BreakHitResult _outhit)) true))
      (:CastFailed
        (Development|PrintString "NotCylidner")))))

(fn Drop
  (bind _mouthgrab (Variables|Default|GetMouthGrab))
  ;[1 1 1] Actually drop
  (Variables|Default|SetIsGrabing false)
  (Class|TogglesInterface|ToggleDrop(Message) (Components|GetOwner (Class|PhysicsHandleComponent|GetGrabbedComponent _mouthgrab)) false)
  (Physics|Components|PhysicsHandle|ReleaseComponent _mouthgrab))

(fn CameraMovement
  (params (input%20mouse :type Float%20%28single-precision%29))
  ;[1 1 1] Camera Rotation On Middle Mouse Button Pressed
  ;;[1 1 1] Relative Location!
  (Transformation|AddRelativeRotation (Variables|Default|GetSpringArm) (Math|Rotator|MakeRotator 0.0 0.0 (Math|Float|Lerp 0.0 1.0 (.yaw (Math|Rotator|MakeRotator 0.0 0.0 input%20mouse)))) false false))

(fn ResetCamera
  ;[1 1 1] We reset the rotation , but keep the height
  (Transformation|SetRelativeRotation (Variables|Default|GetSpringArm) "-35.000000, 0, 0" false false))

(fn Bark
  (bind _returnvalue (Game|Player|GetPlayerPawn 0))
  (Variables|Default|SetIsBarking true)
  (Class|Actor|MakeNoise 1.0 _returnvalue (Transformation|GetActorLocation _returnvalue) 0.0 "None")
  (Audio|Components|Audio|Play (Variables|Default|GetBarkAudio) 0.0))