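; Mobile dog character that mouth-grabs physics Cylinders for points, drops them, and fires a radial-force horn impulse.
; Grab sphere-traces from the mouth into a physics grab whose target follows GrabLocation each tick.
; Tick also compares planar dog-to-human-camera distance, raising game mode energy inside RadiusBorder and draining it beyond CatchBorder.
; CameraBlockingVolume overlaps toggle spring arm collision testing; sprint speed and camera rotation logic are disconnected.
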(event OnComponentActivated(SpringArm)
  (params (Component :type Actor%20Component%20Object%20Reference) (bReset :type Boolean)))

(event OnComponentBeginOverlap(CamerraCollision)
  (params (OverlappedComponent :type Primitive%20Component%20Object%20Reference) (OtherActor :type Actor%20Object%20Reference) (OtherComp :type Primitive%20Component%20Object%20Reference) (OtherBodyIndex :type Integer) (bFromSweep :type Boolean) (SweepResult :type Hit%20Result%20Structure%20%28by%20ref%29))
  (bind _returnvalue (Utilities|GetClass OtherActor))
  (if (== _returnvalue "/Script/Engine.CameraBlockingVolume")
    (Development|PrintString (Utilities|GetClassDisplayName _returnvalue))
    (Variables|/Script/Engine.SpringArmComponent|SetbDoCollisionTest (Variables|Default|GetSpringArm) true)))

(event OnComponentEndOverlap(CamerraCollision)
  (params (OverlappedComponent :type Primitive%20Component%20Object%20Reference) (OtherActor :type Actor%20Object%20Reference) (OtherComp :type Primitive%20Component%20Object%20Reference) (OtherBodyIndex :type Integer))
  (bind _returnvalue (Utilities|GetClass OverlappedComponent))
  (if (== _returnvalue "/Script/Engine.CameraBlockingVolume")
    (Development|PrintString (Utilities|GetClassDisplayName _returnvalue))
    (Variables|/Script/Engine.SpringArmComponent|SetbDoCollisionTest (Variables|Default|GetSpringArm) false)))

(event Custom|CompareCameraAndDogLocation
  ;[0.4002 1 0.3448] Energy By Radius
  ;;[1 1 1] Compare Camera and charecter location
  (bind _output_get (Variables|Default|SetCameraAndDogDistance (- (Variables|Default|GetHumanCameraLocation) (Transformation|GetWorldLocation (Variables|Character|GetMesh)))))
  (bind _output_get_2 (Variables|Default|SetAllTogetherDistance (Math|Float|Sqrt (+ (Math|Float|Square (Math|Float|Absolute(Float) (.x _output_get))) (Math|Float|Square (Math|Float|Absolute(Float) (.y _output_get)))))))
  ;;;[1 1 1] Compare Camera and charecter location
  (if (> _output_get_2 (Variables|Default|GetRadiusBorder))
    (if (> (Variables|Default|GetAllTogetherDistance) (Variables|Default|GetCatchBorder))
      (Variables|Default|SetIsInsideRadius false)
      ;;;[1 1 1] Reduce energy
      (if (>= (- (Variables|/Game/Shenanidog/BluePrints/GameFiles/BP_Game_Mode_Base.BP_Game_Mode_Base_C|GetEnergyAmount (Variables|Default|GetBP_GameMode%20ref)) (Variables|Default|GetEnergy%20to%20Reduce)) 0.0)
        (Variables|/Game/Shenanidog/BluePrints/GameFiles/BP_Game_Mode_Base.BP_Game_Mode_Base_C|SetEnergyAmount (Variables|Default|GetBP_GameMode%20ref) (- (Variables|/Game/Shenanidog/BluePrints/GameFiles/BP_Game_Mode_Base.BP_Game_Mode_Base_C|GetEnergyAmount (Variables|Default|GetBP_GameMode%20ref)) (Variables|Default|GetEnergy%20to%20Reduce)))
        (Default|UpdateUI (Variables|Default|GetBP_GameMode%20ref))))
    (else
      (Variables|Default|SetIsInsideRadius true)
      ;;[1 1 1] Add energy
      (if (<= (+ (Variables|/Game/Shenanidog/BluePrints/GameFiles/BP_Game_Mode_Base.BP_Game_Mode_Base_C|GetEnergyAmount (Variables|Default|GetBP_GameMode%20ref)) (Variables|Default|GetEnergy%20to%20Add)) (+ (Variables|/Game/Shenanidog/BluePrints/GameFiles/BP_Game_Mode_Base.BP_Game_Mode_Base_C|GetMaxEnergyAmount (Variables|Default|GetBP_GameMode%20ref)) 2e+01))
        (Variables|/Game/Shenanidog/BluePrints/GameFiles/BP_Game_Mode_Base.BP_Game_Mode_Base_C|SetEnergyAmount (Variables|Default|GetBP_GameMode%20ref) (+ (Variables|/Game/Shenanidog/BluePrints/GameFiles/BP_Game_Mode_Base.BP_Game_Mode_Base_C|GetEnergyAmount (Variables|Default|GetBP_GameMode%20ref)) (Variables|Default|GetEnergy%20to%20Add)))
        (Default|UpdateUI (Variables|Default|GetBP_GameMode%20ref))))))

(event Custom|CustomEvent
  (params (DeltaSeconds :type Float%20%28single-precision%29))
  ;[1 1 1] UpdateGrabLocation every frame - mouth grab - grab location
  (Physics|Components|PhysicsHandle|SetTargetLocation (Variables|Default|GetMouthGrab) (Transformation|GetWorldLocation (Variables|Default|GetGrabLocation))))

(event EventBeginPlay
  ;[1 1 1] Cast to BP_GameMode
  (bind _asbp_game_mode_base (Utilities|Casting|CastToBP_Game_Mode_Base (Game|GetGameMode)))
  (Variables|Default|SetBP_GameMode%20ref _asbp_game_mode_base))

(event Collision|EventActorBeginOverlap
  (params (OtherActor :type Actor%20Object%20Reference)))

(event EventTick
  (params (DeltaSeconds :type Float%20%28single-precision%29))
  ;[1 1 1] UpdateGrabLocation every frame - mouth grab - grab location
  (Physics|Components|PhysicsHandle|SetTargetLocation (Variables|Default|GetMouthGrab) (Transformation|GetWorldLocation (Variables|Default|GetGrabLocation)))
  (CallFunction|CompareCameraandDogLocation)
  (Utilities|FlowControl|Delay 0.2)
  (Rendering|SetVisibility (Variables|Default|GetCursorToWorld) false false))

(fn ConstructionScript)

(fn UpdateMovementSpeed)

(fn BlowHorn
  ;[1 1 1] Blow Force Event
  (Class|RadialForceComponent|FireImpulse (Variables|Default|GetRadialForce)))

(fn Grab
  (bind _mouthforgrab (Variables|Default|GetMouthForGrab))
  (bind _mesh (Variables|Character|GetMesh))
  (bind _returnvalue (Transformation|GetWorldLocation _mouthforgrab))
  ;[1 1 1] We recognize from sphere of trace for object , what did we hit , and move the hit object to the grab component
  (bind (_outhit _returnvalue_2) (Collision|SphereTraceForObjects _returnvalue (+ _returnvalue (* (Math|Vector|GetForwardVector _mouthforgrab) 5e+01)) 5e+01 (Utilities|Array|MakeArray "ObjectTypeQuery4") false 0 "None"))
  (if _returnvalue_2
    (bind _ascylinders (Utilities|Casting|CastToCylinders (.HitActor (Collision|BreakHitResult _outhit)))
      (:then
        (Variables|Default|SetCylindersRef 0)
        (Class|PhysicsHandleComponent|GrabComponentatLocation (Variables|Default|GetMouthGrab) (.HitComponent (Collision|BreakHitResult _outhit)) (Class|SkinnedMeshComponent|GetBoneName _mesh (Class|SkinnedMeshComponent|GetBoneIndex _mesh "mouth")) (Transformation|GetWorldLocation (.HitComponent (Collision|BreakHitResult _outhit))))
        ;;[1 1 1] This is if we dont want the object we grab colliding with use
        (Collision|SetCollisionResponsetoChannel (.HitComponent (Collision|BreakHitResult _outhit)) "ECC_Pawn" "ECR_Ignore")
        (Variables|Default|SetIsGrabing true)
        (Default|UpdatetheUIforScore _ascylinders (Variables|/Game/Shenanidog/BluePrints/Objects/Cylinders.Cylinders_C|GetPointsForGrab _ascylinders))
        (Class|TogglesInterface|ToggleGrab(Message) (.HitActor (Collision|BreakHitResult _outhit)) true))
      (:CastFailed
        (Development|PrintString "NotCylidner")))))

(fn Drop
  (bind _mouthgrab (Variables|Default|GetMouthGrab))
  ;[1 1 1] Actually drop
  (Variables|Default|SetIsGrabing false)
  (Class|TogglesInterface|ToggleDrop(Message) (Components|GetOwner (Class|PhysicsHandleComponent|GetGrabbedComponent _mouthgrab)) false)
  (Physics|Components|PhysicsHandle|ReleaseComponent _mouthgrab))

(fn CameraMovement
  (params (input%20mouse :type Float%20%28single-precision%29))
  ;[1 1 1] Camera Rotation On Middle Mouse Button Pressed
)

(fn ResetCamera
  ;[1 1 1] We reset the rotation , but keep the height
)