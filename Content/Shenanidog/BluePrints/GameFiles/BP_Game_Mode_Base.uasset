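; Base game mode Blueprint for Shenanidog, where only CalculateScore, which adds points to TotalPoints, has working logic.
; BeginPlay, Tick, UpdateUI and SetTimer are empty events, with their former logic left disconnected.
; That unused logic creates the HUD and Key_Press widgets, pushes energy and points to the UI, and runs a minute/second countdown that toggles win/lose and stops player movement.
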(event Custom|UpdateUI)

(event Custom|SetTimer)

(event EventBeginPlay)

(event EventTick
  (params (DeltaSeconds :type Float%20%28single-precision%29)))

(fn ConstructionScript)

(fn CalculateScore
  (params (Points :type Integer))
  (Variables|Default|SetTotalPoints (+ Points (Variables|Default|GetTotalPoints))))