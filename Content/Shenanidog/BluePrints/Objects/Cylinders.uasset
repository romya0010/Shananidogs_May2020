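; Cylinders is a prop the player's dog can grab and drop in Shenanidog.
; Tick outlines it through custom depth within a player-distance band and, from grab state, adjusts collision with the dog's grab sphere, mass and release prompt.
; Grab/drop interface events and mesh hits set those state flags.
; Scoring, overlap-based tick toggling and UI reference setup are disconnected, so UIREFERENCE is never assigned here.
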(event OnComponentHit(Mesh)
  (params (HitComponent :type Primitive%20Component%20Object%20Reference) (OtherActor :type Actor%20Object%20Reference) (OtherComp :type Primitive%20Component%20Object%20Reference) (NormalImpulse :type Vector :default "0, 0, 0") (Hit :type Hit%20Result%20Structure%20%28by%20ref%29))
  ;[1 1 1] Points for just bumping to stuff
  ;;[1 1 1] Turning Romys light off (only visible :P not in real life) and destroying text
  (Variables|Default|SetHasBeenTouched true)
  (Rendering|SetRenderCustomDepth (Variables|Default|GetMesh%20) false)
  (Variables|Default|SetToDestroyText true))

(event OnComponentBeginOverlap(CollisionTriggerAroundMesh)
  (params (OverlappedComponent :type Primitive%20Component%20Object%20Reference) (OtherActor :type Actor%20Object%20Reference) (OtherComp :type Primitive%20Component%20Object%20Reference) (OtherBodyIndex :type Integer) (bFromSweep :type Boolean) (SweepResult :type Hit%20Result%20Structure%20%28by%20ref%29))
  ;[1 1 1] Tick On \ Off - Disabled
)

(event OnComponentEndOverlap(CollisionTriggerAroundMesh)
  (params (OverlappedComponent :type Primitive%20Component%20Object%20Reference) (OtherActor :type Actor%20Object%20Reference) (OtherComp :type Primitive%20Component%20Object%20Reference) (OtherBodyIndex :type Integer))
  ;[1 1 1] Tick On \ Off - Disabled
)

(event OnBeginCursorOver(Mesh)
  (params (TouchedComponent :type Primitive%20Component%20Object%20Reference))
  ;[1 1 1] TESTSTSTSTST
)

(event OnEndCursorOver(Mesh)
  (params (TouchedComponent :type Primitive%20Component%20Object%20Reference))
  ;[1 1 1] TESTSTSTSTST
  (Rendering|Material|SetScalarParameterValueonMaterials (Variables|Default|GetMesh%20) "Selected" 0.0)
  (Class|TogglesInterface|ToggleHighlight(Message) (Variables|Default|GetUI_REFERENCE) false))

(event Custom|CompareDistToActorAndHighlight
  (bind _returnvalue (Game|GetPlayerCharacter 0))
  (bind _mesh_ (Variables|Default|GetMesh%20))
  (bind _mesh__2 (Variables|Default|GetMesh%20))
  (bind _returnvalue_2 (Transformation|GetWorldLocation _mesh_))
  (bind _mesh (Variables|/Script/Engine.Character|GetMesh _returnvalue))
  (bind _returnvalue_3 (Transformation|GetWorldLocation _mesh))
  (bind _returnvalue_4 (- _returnvalue_2 _returnvalue_3))
  (bind _returnvalue_5 (Math|Vector|VectorLength _returnvalue_4))
  ;[1 1 1] Compare distance from player and highlight
  (if (and (>= _returnvalue_5 (Variables|Default|GetHighlight_Min_Distance)) (< _returnvalue_5 (Variables|Default|GetHighlight_Max_Distance)))
    (Rendering|SetRenderCustomDepth _mesh__2 true)
    (else
      (Rendering|SetRenderCustomDepth _mesh__2 false))))

(event Custom|Update%20the%20UI%20for%20Score
  (params (Points :type Integer))
  ;[1 1 1] Update UI for Score
)

(event EventToggleDrop
  (params (ToggleDrop :type Boolean))
  ;[1 1 1] Interfaces to know grab and drop - it is comming from the Character after the grab / drop function
  (Variables|Default|SetIsGrabbed ToggleDrop)
  (Variables|Default|SetWasDropped true)
  (Variables|Default|SetHasBeenTouched true))

(event EventToggleGrab
  (params (ToggleGrab :type Boolean))
  ;[1 1 1] Interfaces to know grab and drop - it is comming from the Character after the grab / drop function
  (Variables|Default|SetIsGrabbed ToggleGrab)
  (Variables|Default|SetHasBeenTouched true))

(event EventTick
  (params (DeltaSeconds :type Float%20%28single-precision%29))
  ;[1 1 1] Romy's countor light
  (CallFunction|CompareDisttoActorandHighlight)
  ;[1 1 1] setting the collision not to the dog but to the sphere of the dog - collision for grab on and off
  (if (Variables|Default|GetIsGrabbed)
    (Collision|SetCollisionResponsetoChannel (Variables|Default|GetMesh%20) (Collision|GetCollisionObjectType (Variables|/Game/Shenanidog/BluePrints/Character/BluePrints/Dog_Chracter_3rdP.Dog_Chracter_3rdP_C|GetCollisionForGrab (Variables|Default|GetCharacterRef))) "ECR_Block")
    (Class|PrimitiveComponent|SetMassOverrideinKg (Variables|Default|GetMesh%20) "None" (Variables|Default|GetMassWhileGrabbed) true)
    (if (Variables|Default|GetWasDropped)
      (Class|PrimitiveComponent|SetMassOverrideinKg (Variables|Default|GetMesh%20) "None" (Variables|Default|GetMassNotGrabbed) true)
      (else
        (Class|TogglesInterface|ToggleRelease(Message) (Variables|Default|GetUI_REFERENCE) true)))
    (else
      (Collision|SetCollisionResponsetoChannel (Variables|Default|GetMesh%20) "ECC_WorldDynamic" "ECR_Block")
      (if (Variables|Default|GetHasBeenTouched)
        (Class|PrimitiveComponent|SetMassOverrideinKg (Variables|Default|GetMesh%20) "None" (Variables|Default|GetMassNotGrabbed) true)
        (Class|TogglesInterface|ToggleRelease(Message) (Variables|Default|GetUI_REFERENCE) false)))))

(event EventBeginPlay
  ;[1 1 1] Cast to BP_GameMode
  (bind _asdog_chracter_3rd_p (Utilities|Casting|CastToDog_Chracter_3rdP (Game|GetPlayerCharacter 0)))
  (Variables|Default|SetCharacterRef _asdog_chracter_3rd_p)
  (bind _asbp_game_mode_base (Utilities|Casting|CastToBP_Game_Mode_Base (Game|GetGameMode)))
  (Variables|Default|SetBP%20Game%20Mode%20Ref _asbp_game_mode_base))

(fn ConstructionScript)