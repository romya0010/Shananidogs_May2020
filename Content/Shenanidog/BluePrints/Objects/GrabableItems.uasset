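; Base Blueprint for a physical item that a character can grab and drop.
; ToggleGrab and ToggleDrop interface events from the character set grabbed, dropped and touched flags.
; Tick reads those flags every frame to block the character's grab-collision channel or WorldDynamic and to override mesh mass between grabbed and released values.
; Hovering the cursor over the mesh prints a debug string.
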(event OnBeginCursorOver(Mesh)
  (params (TouchedComponent :type Primitive%20Component%20Object%20Reference))
  (Development|PrintString "Hello"))

(event EventToggleDrop
  (params (ToggleDrop :type Boolean))
  ;[1 1 1] Interfaces to know grab and drop - it is comming from the Character after the grab / drop function
  (Variables|Default|SetIsGrabbed ToggleDrop)
  (Variables|Default|SetWasDropped true)
  (Variables|Default|SetHasBeenTouched true))

(event EventToggleGrab
  (params (ToggleGrab :type Boolean))
  ;[1 1 1] Interfaces to know grab and drop - it is comming from the Character after the grab / drop function
  (Variables|Default|SetIsGrabbed ToggleGrab)
  (Variables|Default|SetHasBeenTouched true))

(event EventTick
  (params (DeltaSeconds :type Float%20%28single-precision%29))
  (|CallParentFunction DeltaSeconds)
  (if (Variables|Default|GetIsGrabbed)
    (Collision|SetCollisionResponsetoChannel (Variables|Default|GetMesh%20) (Collision|GetCollisionObjectType (Variables|/Game/Shenanidog/BluePrints/Character/BluePrints/Dog_Character_Mobile.Dog_Character_Mobile_C|GetCollisionForGrab (Variables|Default|GetCharacterRef))) "ECR_Block")
    (Class|PrimitiveComponent|SetMassOverrideinKg (Variables|Default|GetMesh%20) "None" (Variables|Default|GetMassWhileGrabbed) true)
    (if (Variables|Default|GetWasDropped)
      (Class|PrimitiveComponent|SetMassOverrideinKg (Variables|Default|GetMesh%20) "None" (Variables|Default|GetMassNotGrabbed) true))
    (else
      (Collision|SetCollisionResponsetoChannel (Variables|Default|GetMesh%20) "ECC_WorldDynamic" "ECR_Block")
      (if (Variables|Default|GetHasBeenTouched)
        (Class|PrimitiveComponent|SetMassOverrideinKg (Variables|Default|GetMesh%20) "None" (Variables|Default|GetMassNotGrabbed) true)))))

(event EventBeginPlay
  (|CallParentFunction) ; This node is disabled and will not be called.\nDrag off pins to build functionality.
)

(event Collision|EventActorBeginOverlap
  (params (OtherActor :type Actor%20Object%20Reference)))

(fn ConstructionScript
  (|CallParentFunction))