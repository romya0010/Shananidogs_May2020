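; Grabbable cylinder prop in Shenanidog that awards points when first bumped by a tagged component while the dog is outside its radius.
; Tick starts disabled; both Box overlap begin and end events enable it.
; Tick highlights the untouched prop via custom depth within a distance band and adjusts collision and mass for grab state.
; Grab/drop events from the character mark it touched; scoring goes through the game mode, which updates the UI.
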(event OnComponentHit(Cylinder)
  (params (HitComponent :type Primitive%20Component%20Object%20Reference) (OtherActor :type Actor%20Object%20Reference) (OtherComp :type Primitive%20Component%20Object%20Reference) (NormalImpulse :type Vector :default "0, 0, 0") (Hit :type Hit%20Result%20Structure%20%28by%20ref%29))
  ;[1 1 1] Points for just bumping to stuff
  (for _array_element (Variables|/Script/Engine.ActorComponent|GetComponentTags OtherComp)
    _)
  (if (Utilities|Name|Equal(Name) (Utilities|Name|MakeLiteralName _array_element) (GameplayTags|GetTagName (GameplayTags|MakeLiteralGameplayTag)))
    (if (Math|Boolean|NotEqual(Boolean) (Variables|Default|GetHasBeenTouched) true)
      (if (not (Variables|/Game/Shenanidog/BluePrints/Character/BluePrints/Dog_Character.Dog_Character_C|GetIsInsideRadius (Variables|Default|GetCharacterRef)))
        (CallFunction|UpdatetheUIforScore (Variables|Default|GetPointsGeneral))
        ;;[1 1 1] Turning Romys light off (only visible :P not in real life) and destroying text
        (Variables|Default|SetHasBeenTouched true)
        (Rendering|SetRenderCustomDepth (Variables|Default|GetCylinder) false)
        (Variables|Default|SetToDestroyText true)))
    (else
      (Development|PrintString "IhitSomethingElse"))))

(event OnComponentBeginOverlap(Box)
  (params (OverlappedComponent :type Primitive%20Component%20Object%20Reference) (OtherActor :type Actor%20Object%20Reference) (OtherComp :type Primitive%20Component%20Object%20Reference) (OtherBodyIndex :type Integer) (bFromSweep :type Boolean) (SweepResult :type Hit%20Result%20Structure%20%28by%20ref%29))
  ;[1 1 1] Tick On \ Off
  (if (not (Variables|/Game/Shenanidog/BluePrints/Character/BluePrints/Dog_Character.Dog_Character_C|GetIsInsideRadius (Variables|Default|GetCharacterRef)))
    (if (== (Utilities|GetClass (Variables|Default|GetCharacterRef)) (Utilities|GetClass OtherActor))
      (Actor|Tick|SetActorTickEnabled true))))

(event OnComponentEndOverlap(Box)
  (params (OverlappedComponent :type Primitive%20Component%20Object%20Reference) (OtherActor :type Actor%20Object%20Reference) (OtherComp :type Primitive%20Component%20Object%20Reference) (OtherBodyIndex :type Integer))
  ;[1 1 1] Tick On \ Off
  (if (== (Utilities|GetClass (Variables|Default|GetCharacterRef)) (Utilities|GetClass OtherActor))
    (Actor|Tick|SetActorTickEnabled true)))

(event Custom|CompareDistToActorAndHighlight
  (bind _returnvalue (Game|GetPlayerCharacter 0))
  (bind _cylinder (Variables|Default|GetCylinder))
  (bind _cylinder_2 (Variables|Default|GetCylinder))
  (bind _returnvalue_2 (Transformation|GetWorldLocation _cylinder))
  (bind _mesh (Variables|/Script/Engine.Character|GetMesh _returnvalue))
  (bind _returnvalue_3 (Transformation|GetWorldLocation _mesh))
  (bind _returnvalue_4 (- _returnvalue_2 _returnvalue_3))
  (bind _returnvalue_5 (Math|Vector|VectorLength _returnvalue_4))
  ;[1 1 1] Compare distance from player and highlight
  (if (and (>= _returnvalue_5 (Variables|Default|GetHighlight_Min_Distance)) (< _returnvalue_5 (Variables|Default|GetHighlight_Max_Distance)))
    (if (not (Variables|Default|GetHasBeenTouched))
      (Rendering|SetRenderCustomDepth _cylinder_2 true)
      (if (Math|Boolean|Equal(Boolean) (Variables|Default|GetToDestroyText) false)
        _))
    (else
      (Rendering|SetRenderCustomDepth _cylinder_2 false)
      (if (Math|Boolean|Equal(Boolean) (Variables|Default|GetToDestroyText) false)
        _))))

(event Custom|Update%20the%20UI%20for%20Score
  (params (Points :type Integer))
  (bind _bp_game_mode_ref (Variables|Default|GetBP%20Game%20Mode%20Ref))
  ;[1 1 1] Update UI for Score
  (if (or (Variables|Default|GetIsGrabbed) (Math|Boolean|NotEqual(Boolean) (Variables|Default|GetHasBeenTouched) true))
    (Default|CalculateScore _bp_game_mode_ref Points)
    (Default|UpdateUI _bp_game_mode_ref)
    (Variables|Default|SetHasBeenTouched true)))

(event EventToggleDrop
  (params (ToggleDrop :type Boolean))
  ;[1 1 1] Interfaces to know grab and drop - it is comming from the Character after the grab / drop function
  (Variables|Default|SetIsGrabbed ToggleDrop)
  (Variables|Default|SetWasDropped true)
  (Variables|Default|SetHasBeenTouched true))

(event EventToggleGrab
  (params (ToggleGrab :type Boolean))
  ;[1 1 1] Interfaces to know grab and drop - it is comming from the Character after the grab / drop function
  (Variables|Default|SetIsGrabbed ToggleGrab)
  (Variables|Default|SetHasBeenTouched true)
  (Rendering|SetRenderCustomDepth (Variables|Default|GetCylinder) false))

(event EventTick
  (params (DeltaSeconds :type Float%20%28single-precision%29))
  ;[1 1 1] Setting Text Location Above the mesh and hiding it
  ;[1 1 1] Romy's countor light
  (CallFunction|CompareDisttoActorandHighlight)
  ;[1 1 1] setting the collision not to the dog but to the sphere of the dog - collision for grab on and off
  (if (Variables|Default|GetIsGrabbed)
    (Collision|SetCollisionResponsetoChannel (Variables|Default|GetCylinder) (Collision|GetCollisionObjectType (Variables|/Game/Shenanidog/BluePrints/Character/BluePrints/Dog_Character.Dog_Character_C|GetCollisionForGrab (Variables|Default|GetCharacterRef))) "ECR_Block")
    (Class|PrimitiveComponent|SetMassOverrideinKg (Variables|Default|GetCylinder) "None" (Variables|Default|GetMassWhileGrabbed) true)
    (if (Variables|Default|GetWasDropped)
      (Class|PrimitiveComponent|SetMassOverrideinKg (Variables|Default|GetCylinder) "None" (Variables|Default|GetMassNotGrabbed) true))
    (else
      (Collision|SetCollisionResponsetoChannel (Variables|Default|GetCylinder) "ECC_WorldDynamic" "ECR_Block")
      (if (Variables|Default|GetHasBeenTouched)
        (Class|PrimitiveComponent|SetMassOverrideinKg (Variables|Default|GetCylinder) "None" (Variables|Default|GetMassNotGrabbed) true)))))

(event EventBeginPlay
  ;[1 1 1] Cast to BP_GameMode
  (bind _asdog_character (Utilities|Casting|CastToDog_Character (Game|GetPlayerCharacter 0)))
  (Variables|Default|SetCharacterRef _asdog_character)
  (bind _asbp_game_mode_base (Utilities|Casting|CastToBP_Game_Mode_Base (Game|GetGameMode)))
  (Variables|Default|SetBP%20Game%20Mode%20Ref _asbp_game_mode_base)
  (Actor|Tick|SetActorTickEnabled false))

(fn ConstructionScript)